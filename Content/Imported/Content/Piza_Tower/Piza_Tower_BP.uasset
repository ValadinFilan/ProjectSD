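; Pizza tower actor made of three static meshes whose materials animate through a "Slider" scalar parameter while the F key is held.
; The construction script creates a dynamic material instance for each mesh and stores them as Layer1 to Layer3.
; Pressing F prints a debug string and plays the Anim timeline, which drives Slider on all three layers.
; Releasing F reverses the timeline.
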(event EventBeginPlay)

(event Collision|EventActorBeginOverlap
  (params (OtherActor :type Actor%20Object%20Reference)))

(event EventTick
  (params (DeltaSeconds :type Float%20%28single-precision%29)))

(event Input|KeyboardEvents|F
  (params (Key :type Key%20Structure :default "None"))
  (:Pressed
    (Development|PrintString "Hello")
    (bind _newtrack_1 (Timeline|Anim Play)
      (:Update
        (Rendering|Material|SetScalarParameterValue (Variables|Default|Getlayer1) "Slider" _newtrack_1 :!class /Script/Engine.MaterialInstanceDynamic)
        (Rendering|Material|SetScalarParameterValue (Variables|Default|Getlayer2) "Slider" _newtrack_1 :!class /Script/Engine.MaterialInstanceDynamic)
        (Rendering|Material|SetScalarParameterValue (Variables|Default|Getlayer3) "Slider" _newtrack_1 :!class /Script/Engine.MaterialInstanceDynamic))))
  (:Released
    (Timeline|Anim Reverse)))

(fn ConstructionScript
  (bind _staticmesh1 (Variables|Default|GetStaticMesh1))
  (bind _staticmesh2 (Variables|Default|GetStaticMesh2))
  (bind _staticmesh0 (Variables|Default|GetStaticMesh0))
  (bind _returnvalue (Rendering|Material|CreateDynamicMaterialInstance _staticmesh0 0 "/Game/Piza_Tower/layer1.layer1" "None" :!class /Script/Engine.PrimitiveComponent))
  (bind _returnvalue_2 (Rendering|Material|CreateDynamicMaterialInstance _staticmesh1 0 "/Game/Piza_Tower/layer2.layer2" "None" :!class /Script/Engine.PrimitiveComponent))
  (bind _returnvalue_3 (Rendering|Material|CreateDynamicMaterialInstance _staticmesh2 0 "/Game/Piza_Tower/layer3.layer3" "None" :!class /Script/Engine.PrimitiveComponent))
  (Rendering|Material|SetMaterial _staticmesh0 0 _returnvalue)
  (Rendering|Material|SetMaterial _staticmesh1 0 _returnvalue_2)
  (Rendering|Material|SetMaterial _staticmesh2 0 _returnvalue_3)
  (Variables|Default|Setlayer1 _returnvalue)
  (Variables|Default|Setlayer2 _returnvalue_2)
  (Variables|Default|Setlayer3 _returnvalue_3))