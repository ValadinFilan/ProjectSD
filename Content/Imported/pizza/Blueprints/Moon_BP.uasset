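; Moon actor with keyboard-controlled lunar phase and brightness.
; Holding Z or X runs a timeline forward or backward to yaw the Phase component through a half turn, pausing on release.
; Holding C runs a second timeline that drives Phase intensity, with a FlipFlop alternating direction on each press.
; The construction script moves the actor to Center and sets the Sphere's relative location to Center plus OrbitDiameter along Y.
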(event EventBeginPlay)

(event Collision|EventActorBeginOverlap
  (params (OtherActor :type Actor%20Object%20Reference)))

(event EventTick
  (params (DeltaSeconds :type Float%20%28single-precision%29)))

(event Input|KeyboardEvents|Z
  (params (Key :type Key%20Structure :default "None"))
  (:Pressed
    (bind _newtrack_0 (Timeline|Phase%20Changing Play)
      (:Update
        (Transformation|SetRelativeRotation (Variables|Default|GetPhase) (Math|Rotator|MakeRotator 0.0 0.0 (+ (* _newtrack_0 1.8e+02) 9e+01)) false false))))
  (:Released
    (Timeline|Phase%20Changing Stop)))

(event Input|KeyboardEvents|X
  (params (Key :type Key%20Structure :default "None"))
  (:Pressed
    (bind _newtrack_0 (Timeline|Phase%20Changing Reverse)
      (:Update
        (Transformation|SetRelativeRotation (Variables|Default|GetPhase) (Math|Rotator|MakeRotator 0.0 0.0 (+ (* _newtrack_0 1.8e+02) 9e+01)) false false))))
  (:Released
    (Timeline|Phase%20Changing Stop)))

(event Input|KeyboardEvents|C
  (params (Key :type Key%20Structure :default "None"))
  (:Pressed
    (Utilities|FlowControl|FlipFlop
      (:A
        (bind _newtrack_1 (Timeline|Emissioon%20Changing Play)
          (:Update
            (Rendering|Components|Light|SetIntensity (Variables|Default|GetPhase) _newtrack_1))))
      (:B
        (Timeline|Emissioon%20Changing Reverse))))
  (:Released
    (Timeline|Emissioon%20Changing Stop)))

(fn ConstructionScript
  (Transformation|SetActorLocation (Variables|Default|Getcenter) false false)
  (Transformation|SetRelativeLocation (Variables|Default|GetSphere) (+ (Variables|Default|Getcenter) (Math|Vector|MakeVector 0.0 (Variables|Default|GetOrbitDiameter) 0.0)) false false))