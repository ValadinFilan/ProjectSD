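; Pizza tower actor whose three mesh layers respond visually to a changing global value.
; The construction script creates a dynamic material instance for each mesh and stores it in a layer variable.
; On BeginPlay it binds to a global value-changed dispatcher, which drives each material's Slider parameter with the value inverted and normalized against a fixed maximum, without clamping or Tick.
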(event Custom|OnGlobalValueChangedEvent
  (params (Value :type Float%20%28double-precision%29))
  (bind _returnvalue (- 1.3e+04 Value))
  (bind _returnvalue_2 (/ _returnvalue 1.3e+04))
  (Rendering|Material|SetScalarParameterValue (Variables|Default|Getlayer1) "Slider" _returnvalue_2 :!class /Script/Engine.MaterialInstanceDynamic)
  (Rendering|Material|SetScalarParameterValue (Variables|Default|Getlayer2) "Slider" _returnvalue_2 :!class /Script/Engine.MaterialInstanceDynamic)
  (Rendering|Material|SetScalarParameterValue (Variables|Default|Getlayer3) "Slider" _returnvalue_2 :!class /Script/Engine.MaterialInstanceDynamic))

(event EventBeginPlay
  (EventDispatchers|AssignOnGlobalValueChanged (delegate Custom|OnGlobalValueChangedEvent)))

(event Collision|EventActorBeginOverlap
  (params (OtherActor :type Actor%20Object%20Reference)))

(event EventTick
  (params (DeltaSeconds :type Float%20%28single-precision%29)))

(fn ConstructionScript
  (bind _staticmesh1 (Variables|Default|GetStaticMesh1))
  (bind _staticmesh2 (Variables|Default|GetStaticMesh2))
  (bind _staticmesh0 (Variables|Default|GetStaticMesh0))
  (bind _returnvalue (Rendering|Material|CreateDynamicMaterialInstance _staticmesh0 0 "/Game/Materials/layer1.layer1" "None" :!class /Script/Engine.PrimitiveComponent))
  (bind _returnvalue_2 (Rendering|Material|CreateDynamicMaterialInstance _staticmesh1 0 "/Game/Materials/layer2.layer2" "None" :!class /Script/Engine.PrimitiveComponent))
  (bind _returnvalue_3 (Rendering|Material|CreateDynamicMaterialInstance _staticmesh2 0 "/Game/Materials/layer3.layer3" "None" :!class /Script/Engine.PrimitiveComponent))
  (Rendering|Material|SetMaterial _staticmesh0 0 _returnvalue)
  (Rendering|Material|SetMaterial _staticmesh1 0 _returnvalue_2)
  (Rendering|Material|SetMaterial _staticmesh2 0 _returnvalue_3)
  (Variables|Default|Setlayer1 _returnvalue)
  (Variables|Default|Setlayer2 _returnvalue_2)
  (Variables|Default|Setlayer3 _returnvalue_3))