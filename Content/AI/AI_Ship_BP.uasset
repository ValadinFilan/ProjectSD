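; AI ship actor that shuttles back and forth along a referenced spline, starting on BeginPlay.
; A Move timeline, rate-scaled by TimeToComplete, lerps distance along the spline to set location and rotation, adding 180 yaw when Reverse is false.
; At each end, a Rotate timeline turns the ship, then flips Reverse and restarts movement.
; Any actor overlap stops movement, and ending the overlap resumes it in the current direction.
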(event Custom|FollowSpline
  (bind _splineref (Variables|Default|GetSplineREF))
  (bind _spline (Variables|/Game/Blueprints/BP_Spline.BP_Spline_C|GetSpline _splineref))
  (Components|Timeline|SetPlayRate (Variables|Default|GetMove) (/ 1.0 (Variables|Default|GetTime%20to%20complete)))
  (if (Variables|Default|Getreverse)
    (bind _newtrack_0 (Timeline|Move Play)
      (:Update
        (if (Variables|Default|Getreverse)
          (Transformation|SetActorTransform (Math|Transform|MakeTransform (Spline|GetLocationatDistanceAlongSpline _spline (Math|Float|Lerp 0.0 (Spline|GetSplineLength _spline) _newtrack_0) "World") (Spline|GetRotationatDistanceAlongSpline _spline (Math|Float|Lerp 0.0 (Spline|GetSplineLength _spline) _newtrack_0) "Local") "1.000000,1.000000,1.000000"))
          (else
            (Transformation|SetActorTransform (Math|Transform|MakeTransform (Spline|GetLocationatDistanceAlongSpline _spline (Math|Float|Lerp 0.0 (Spline|GetSplineLength _spline) _newtrack_0) "World") (Math|Rotator|MakeRotator (.roll (Spline|GetRotationatDistanceAlongSpline _spline (Math|Float|Lerp 0.0 (Spline|GetSplineLength _spline) _newtrack_0) "Local")) (.pitch (Spline|GetRotationatDistanceAlongSpline _spline (Math|Float|Lerp 0.0 (Spline|GetSplineLength _spline) _newtrack_0) "Local")) (+ (.yaw (Spline|GetRotationatDistanceAlongSpline _spline (Math|Float|Lerp 0.0 (Spline|GetSplineLength _spline) _newtrack_0) "Local")) 1.8e+02)) "1.000000,1.000000,1.000000")))))
      (:Finished
        (Development|PrintString "Hello")
        (Variables|Default|SetcurrRot (Transformation|GetActorRotation))
        (bind _newtrack_1 (Timeline|Rotate PlayFromStart)
          (:Update
            (Transformation|SetActorRotation (Math|Rotator|MakeRotator 0.0 0.0 (+ (.yaw (Variables|Default|GetcurrRot)) (* _newtrack_1 1.8e+02)))))
          (:Finished
            (Variables|Default|Setreverse (not (Variables|Default|Getreverse)))
            (CallFunction|FollowSpline)))))
    (else
      (Timeline|Move Reverse))))

(event EventBeginPlay
  (CallFunction|FollowSpline))

(event Collision|EventActorBeginOverlap
  (params (OtherActor :type Actor%20Object%20Reference))
  (bind _splineref (Variables|Default|GetSplineREF))
  (bind _spline (Variables|/Game/Blueprints/BP_Spline.BP_Spline_C|GetSpline _splineref))
  (bind _newtrack_0 (Timeline|Move Stop)
    (:Update
      (if (Variables|Default|Getreverse)
        (Transformation|SetActorTransform (Math|Transform|MakeTransform (Spline|GetLocationatDistanceAlongSpline _spline (Math|Float|Lerp 0.0 (Spline|GetSplineLength _spline) _newtrack_0) "World") (Spline|GetRotationatDistanceAlongSpline _spline (Math|Float|Lerp 0.0 (Spline|GetSplineLength _spline) _newtrack_0) "Local") "1.000000,1.000000,1.000000"))
        (else
          (Transformation|SetActorTransform (Math|Transform|MakeTransform (Spline|GetLocationatDistanceAlongSpline _spline (Math|Float|Lerp 0.0 (Spline|GetSplineLength _spline) _newtrack_0) "World") (Math|Rotator|MakeRotator (.roll (Spline|GetRotationatDistanceAlongSpline _spline (Math|Float|Lerp 0.0 (Spline|GetSplineLength _spline) _newtrack_0) "Local")) (.pitch (Spline|GetRotationatDistanceAlongSpline _spline (Math|Float|Lerp 0.0 (Spline|GetSplineLength _spline) _newtrack_0) "Local")) (+ (.yaw (Spline|GetRotationatDistanceAlongSpline _spline (Math|Float|Lerp 0.0 (Spline|GetSplineLength _spline) _newtrack_0) "Local")) 1.8e+02)) "1.000000,1.000000,1.000000")))))
    (:Finished
      (Development|PrintString "Hello")
      (Variables|Default|SetcurrRot (Transformation|GetActorRotation))
      (bind _newtrack_1 (Timeline|Rotate PlayFromStart)
        (:Update
          (Transformation|SetActorRotation (Math|Rotator|MakeRotator 0.0 0.0 (+ (.yaw (Variables|Default|GetcurrRot)) (* _newtrack_1 1.8e+02)))))
        (:Finished
          (Variables|Default|Setreverse (not (Variables|Default|Getreverse)))
          (CallFunction|FollowSpline))))))

(event EventTick
  (params (DeltaSeconds :type Float%20%28single-precision%29)))

(event Collision|EventActorEndOverlap
  (params (OtherActor :type Actor%20Object%20Reference))
  (bind _splineref (Variables|Default|GetSplineREF))
  (bind _spline (Variables|/Game/Blueprints/BP_Spline.BP_Spline_C|GetSpline _splineref))
  (if (Variables|Default|Getreverse)
    (bind _newtrack_0 (Timeline|Move Play)
      (:Update
        (if (Variables|Default|Getreverse)
          (Transformation|SetActorTransform (Math|Transform|MakeTransform (Spline|GetLocationatDistanceAlongSpline _spline (Math|Float|Lerp 0.0 (Spline|GetSplineLength _spline) _newtrack_0) "World") (Spline|GetRotationatDistanceAlongSpline _spline (Math|Float|Lerp 0.0 (Spline|GetSplineLength _spline) _newtrack_0) "Local") "1.000000,1.000000,1.000000"))
          (else
            (Transformation|SetActorTransform (Math|Transform|MakeTransform (Spline|GetLocationatDistanceAlongSpline _spline (Math|Float|Lerp 0.0 (Spline|GetSplineLength _spline) _newtrack_0) "World") (Math|Rotator|MakeRotator (.roll (Spline|GetRotationatDistanceAlongSpline _spline (Math|Float|Lerp 0.0 (Spline|GetSplineLength _spline) _newtrack_0) "Local")) (.pitch (Spline|GetRotationatDistanceAlongSpline _spline (Math|Float|Lerp 0.0 (Spline|GetSplineLength _spline) _newtrack_0) "Local")) (+ (.yaw (Spline|GetRotationatDistanceAlongSpline _spline (Math|Float|Lerp 0.0 (Spline|GetSplineLength _spline) _newtrack_0) "Local")) 1.8e+02)) "1.000000,1.000000,1.000000")))))
      (:Finished
        (Development|PrintString "Hello")
        (Variables|Default|SetcurrRot (Transformation|GetActorRotation))
        (bind _newtrack_1 (Timeline|Rotate PlayFromStart)
          (:Update
            (Transformation|SetActorRotation (Math|Rotator|MakeRotator 0.0 0.0 (+ (.yaw (Variables|Default|GetcurrRot)) (* _newtrack_1 1.8e+02)))))
          (:Finished
            (Variables|Default|Setreverse (not (Variables|Default|Getreverse)))
            (CallFunction|FollowSpline)))))
    (else
      (Timeline|Move Reverse))))

(fn ConstructionScript)