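; BP_Ship is a ship that loops along a TrackSpline and changes its mesh with the current epoch.
; Each Tick it derives spline distance from Speed and ParentTimeCore's TimeValue plus TimeOffset, so position follows the shared time value instead of accumulating.
; It adds a lateral Offset and sine-based bobbing and pitch to the spline transform.
; UpdateEpoch swaps between three meshes when the stage changes, also re-transforming the mesh for the third.
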(event EventBeginPlay)

(event EventUpdateEpoch
  (params (EpochNum :type Integer) (VisualisatingValue :type Integer))
  (bind _cube (Variables|Default|GetCube))
  (bind _cube_2 (Variables|Default|GetCube))
  (if (not (== EpochNum (Variables|Default|GetCurentStage)))
    (if (== EpochNum 3)
      (Components|StaticMesh|SetStaticMesh _cube_2 (Variables|Default|GetEpoch3))
      (Transformation|SetRelativeRotation _cube "0,-90.000000, 0" false false)
      (Transformation|SetRelativeScale3D _cube "2.000000,2.000000,2.000000")
      (Transformation|SetRelativeLocation _cube "0, 0,400.000000" false false)
      (Variables|Default|SetCurentStage EpochNum :!label _label)
      (elif (== EpochNum 2)
        (Components|StaticMesh|SetStaticMesh _cube_2 (Variables|Default|GetEpoch2))
        (goto _label)
        (elif (== EpochNum 1)
          (Components|StaticMesh|SetStaticMesh _cube_2 (Variables|Default|GetEpoch1))
          (goto _label))))))

(event EventTick
  (params (DeltaSeconds :type Float%20%28single-precision%29))
  (bind _parenttimecore (Variables|Default|GetParentTimeCore))
  (bind _speed (Variables|Default|GetSpeed))
  (bind _offset (Variables|Default|GetOffset))
  (bind _timeoffset (Variables|EpochesandTime|GetTimeOffset))
  (bind _trackspline (Variables|Default|GetTrackSpline))
  (bind _returnvalue (Transformation|GetActorLocation _trackspline))
  (bind _timevalue (Variables|/Script/SDProject.TimeCore|GetTimeValue _parenttimecore))
  (bind _spline1 (Variables|/Game/Blueprints/BP_Spline.BP_Spline_C|GetSpline1 _trackspline))
  (bind _returnvalue_2 (Spline|GetSplineLength _spline1))
  (bind _returnvalue_3 (+ _timeoffset _timevalue))
  (bind _returnvalue_4 (Math|Float|Round _returnvalue_2))
  (bind _returnvalue_5 (* _speed _returnvalue_3))
  (bind _returnvalue_6 (Math|Integer|%(Integer) _returnvalue_5 _returnvalue_4))
  (bind _returnvalue_7 (Math|Conversions|ToFloat(Integer) _returnvalue_6))
  (bind _returnvalue_8 (Class|SplineComponent|GetRightVectoratDistanceAlongSpline _spline1 _returnvalue_7 "Local"))
  (bind _returnvalue_9 (Spline|GetLocationatDistanceAlongSpline _spline1 _returnvalue_7 "Local"))
  (bind _returnvalue_10 (* _returnvalue_7 0.0005))
  (bind _returnvalue_11 (Math|Trig|Sin(Radians) _returnvalue_10))
  (bind _returnvalue_12 (* _returnvalue_8 _offset))
  (bind _returnvalue_13 (* _returnvalue_11 5e+01))
  (bind _returnvalue_14 (+ _returnvalue _returnvalue_9 _returnvalue_12 (Math|Vector|MakeVector 0.0 0.0 _returnvalue_13)))
  (if (Utilities|IsValid (Variables|Default|GetTrackSpline))
    (Transformation|SetActorLocation (Math|Vector|MakeVector (.x _returnvalue_14) (.y _returnvalue_14) (.z _returnvalue_14)) false true)
    (Transformation|SetActorRotation (Spline|GetRotationatDistanceAlongSpline _spline1 _returnvalue_7 "Local"))
    (Transformation|AddActorLocalRotation (Math|Rotator|MakeRotator 0.0 (* _returnvalue_11 1.0) 0.0) false false)))

(fn ConstructionScript)