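; BP_Road is a road parent actor meant to visualise an epoch-driven change across its attached road and border blocks.
; On BeginPlay it maps each directly attached actor to a random time offset within RoadChangeDuration, for a staggered transition.
; Disconnected logic would fade road-block colours and toggle border cubes from epoch, timeline value and those offsets.
; UpdateEpoch itself is empty, so none of that visual update runs.
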(event EventBeginPlay
  (for _array_element (Actor|GetAttachedActors true false)
    (Utilities|Map|Add (Variables|Default|GetAttachedActors) _array_element (Math|Float|Truncate (* (Math|Random|RandomFloatinRange 0.0 1.0) (Variables|Default|GetRoadChangeDuration))))))

(event Collision|EventActorBeginOverlap
  (params (OtherActor :type Actor%20Object%20Reference)))

(event EventUpdateEpoch
  (params (EpochNum :type Integer) (VisualisatingValue :type Integer)))

(fn ConstructionScript)