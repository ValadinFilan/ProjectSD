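; BP_LightInTime is a light actor that exists only in one time epoch and follows the night cycle.
; On BeginPlay it binds to start-epoch events from ParentTimeCore and night events from ParentLightSystem.
; The actor is visible only when the started epoch matches TargetEpoch, and its point light component is activated at night and deactivated otherwise.
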(event Custom|StartEpochEvent_Event_1
  (params (EpochNum :type Integer))
  (if (== EpochNum (Variables|Default|GetTargetEpoch))
    (Rendering|SetActorHiddenInGame false)
    (else
      (Rendering|SetActorHiddenInGame true))))

(event Custom|TurnOnNightEvent_Event_0
  (params (Night :type Boolean))
  (bind _pointlightcomponent (Variables|Default|GetPointLightComponent))
  (if Night
    (Components|Activation|SetActive _pointlightcomponent true false)
    (else
      (Components|Activation|SetActive _pointlightcomponent false false))))

(event EventBeginPlay
  (EventDispatchers|AssignStartEpochEvent (Utilities|ResolveSoftReference (Variables|Default|GetParentTimeCore)) (delegate Custom|StartEpochEvent_Event_1))
  (EventDispatchers|AssignTurnonNightEvent (Utilities|ResolveSoftReference (Variables|Default|GetParentLightSystem)) (delegate Custom|TurnOnNightEvent_Event_0)))

(event EventTick
  (params (DeltaSeconds :type Float%20%28single-precision%29)))

(fn ConstructionScript)