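; BP_TransportManager is an actor that populates the level with cars on spline tracks according to the current epoch.
; StartEpoch fills the pool to one past MaxActors when the epoch is above 2, and otherwise destroys all spawned actors.
; SpawnNewCar spawns a random class, passes on ParentTimeCore, and assigns a random time offset plus a track and offset drawn independently from the Splines map's keys and values.
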(event EventBeginPlay)

(event Collision|EventActorBeginOverlap
  (params (OtherActor :type Actor%20Object%20Reference)))

(event EventTick
  (params (DeltaSeconds :type Float%20%28single-precision%29)))

(event EventStartEpoch
  (params (EpochNum :type Integer))
  (bind _actors (Variables|Default|GetActors))
  (bind _output (Utilities|Array|Get(acopy) _actors))
  (if (> EpochNum 2)
    (while (<= (Utilities|Array|Length (Variables|Default|GetActors)) (Variables|Default|GetMaxActors))
      (CallFunction|SpawnNewCar))
    (else
      (while (> (Utilities|Array|Length (Variables|Default|GetActors)) 0)
        (bind _output_get (Variables|Default|SetDestroyActor _output))
        (Utilities|Array|RemoveItem (Variables|Default|GetActors) _output)
        (Actor|DestroyActor _output_get)))))

(fn ConstructionScript)

(fn SpawnNewCar
  (bind _actor_refs (Variables|Default|GetActor%20refs))
  (bind _splines (Variables|Default|GetSplines))
  (bind _returnvalue (Utilities|Map|Length _splines))
  (bind _returnvalue_2 (- _returnvalue 1))
  (bind _returnvalue_3 (Math|Random|RandomIntegerinRange 0 _returnvalue_2))
  (bind _returnvalue_4 (Game|SpawnActorfromClass (Utilities|Array|Get(acopy) _actor_refs (Math|Random|RandomIntegerinRange 0 (- (Utilities|Array|Length _actor_refs) 1))) (Transformation|GetActorTransform) "AlwaysSpawn" 0 0))
  (bind _keys (Utilities|Map|Keys _splines))
  (bind _values (Utilities|Map|Values _splines))
  (Variables|/Game/Blueprints/BP_Car.BP_Car_C|SetTrackSpline _returnvalue_4 (Utilities|Array|Get(acopy) _keys _returnvalue_3))
  (Variables|/Game/Blueprints/BP_Car.BP_Car_C|SetOffset _returnvalue_4 (Utilities|Array|Get(acopy) _values _returnvalue_3))
  (Variables|/Game/Blueprints/BP_Car.BP_Car_C|SetTimeOffset _returnvalue_4 (* (Math|Random|RandomIntegerinRange 0 100) 10))
  (Utilities|Array|Add (Variables|Default|GetActors) _returnvalue_4)
  (Variables|/Script/SDProject.ActorSynchronizedWithTime|SetParentTimeCore _returnvalue_4 (Variables|Default|GetParentTimeCore)))