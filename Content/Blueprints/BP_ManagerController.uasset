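; BP_ManagerController is a player controller that shows a management widget and switches between game and UI input.
; On BeginPlay it creates BP_ManageWidget, adds it to the viewport and starts in game-only input mode.
; The Tab key toggles between game-only and game-and-UI input, tracking the state in a boolean and showing or hiding the mouse cursor to match.
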(event EventBeginPlay
  (bind _returnvalue (Game|ConstructObjectfromClass "/Game/Blueprints/BP_ManageWidget.BP_ManageWidget_C"))
  (UserInterface|Viewport|AddtoViewport _returnvalue 0)
  (Input|SetInputModeGameOnly self)
  (Variables|Default|SetInputGameMode true))

(event EventTick
  (params (DeltaSeconds :type Float%20%28single-precision%29)))

(event Input|KeyboardEvents|Tab
  (params (Key :type Key%20Structure :default "None"))
  (bind _self self)
  (:Pressed
    (if (Variables|Default|GetInputGameMode)
      (Input|SetInputModeGameandUI _self 0 "DoNotLock" true)
      (Variables|Default|SetInputGameMode false)
      (Variables|Default|SetbShowMouseCursor true)
      (else
        (Input|SetInputModeGameOnly _self)
        (Variables|Default|SetInputGameMode true)
        (Variables|Default|SetbShowMouseCursor false)))))

(fn ConstructionScript)