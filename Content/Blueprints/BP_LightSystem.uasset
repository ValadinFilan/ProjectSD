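; BP_LightSystem drives a day/night cycle by rotating the Sun and Moon actors from the parent time core's clock.
; Each tick, it wraps the time by the speed-scaled day duration and passes it to GetAngle for a cycle angle.
; RotateLight applies that angle as Sun pitch and, offset half a turn, as Moon roll.
; It also calls TurnOnNightEvent every tick, true through the first half-turn and false afterwards.
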(event EventBeginPlay)

(event Collision|EventActorBeginOverlap
  (params (OtherActor :type Actor%20Object%20Reference)))

(event EventTick
  (params (DeltaSeconds :type Float%20%28single-precision%29))
  (bind _defaultduration (Variables|Default|GetDefaultDuration))
  (bind _speed (Variables|Default|GetSpeed))
  (bind _parenttimecore (Variables|Default|GetParentTimeCore))
  (bind _returnvalue (/ _defaultduration _speed))
  (bind _timevalue (Variables|/Script/SDProject.TimeCore|GetTimeValue _parenttimecore))
  (bind _returnvalue_2 (Math|Integer|%(Integer) _timevalue _returnvalue))
  (bind _angle (Utilities|GetAngle _returnvalue_2 _returnvalue))
  (CallFunction|RotateLight _angle)
  (if (< 1.8e+02 _angle)
    (Default|CallTurnonNightEvent false)
    (else
      (Default|CallTurnonNightEvent true))))

(fn ConstructionScript)

(fn RotateLight
  (params (Angle :type Float%20%28double-precision%29))
  (bind _sun (Variables|Default|GetSun))
  (bind _moon (Variables|Default|GetMoon))
  (if (Utilities|IsValid (Utilities|ResolveSoftReference _sun))
    (Transformation|SetActorRotation (Utilities|ResolveSoftReference _sun) (Math|Rotator|MakeRotator 0.0 Angle 0.0)))
  (if (Utilities|IsValid (Utilities|ResolveSoftReference _moon))
    (Transformation|SetActorRotation (Utilities|ResolveSoftReference _moon) (Math|Rotator|MakeRotator (+ Angle 1.8e+02) 0.0 0.0))))