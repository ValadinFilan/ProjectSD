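; Base light object actor that responds to a parent light system's night events and can appear only in a target epoch.
; On BeginPlay it registers TurnOnNightEvent with a valid ParentLightSystem, forwarding the Night value to TurnOnLight, which is an empty stub here.
; When InTime is set, StartEpoch shows the actor in its TargetEpoch and hides it in any other.
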(event Custom|TurnOnNightEvent
  (params (Night :type Boolean))
  (CallFunction|TurnonLight Night))

(event EventBeginPlay
  (bind _parentlightsystem (Variables|LightSystem|GetParentLightSystem))
  (if (Utilities|IsValid _parentlightsystem)
    (EventDispatchers|AssignTurnonNightEvent _parentlightsystem (delegate Custom|TurnOnNightEvent))))

(event Collision|EventActorBeginOverlap
  (params (OtherActor :type Actor%20Object%20Reference)))

(event EventTick
  (params (DeltaSeconds :type Float%20%28single-precision%29)))

(event EventStartEpoch
  (params (EpochNum :type Integer))
  (if (Variables|Default|GetInTime)
    (if (== EpochNum (Variables|Default|GetTargetEpoch))
      (Rendering|SetActorHiddenInGame false)
      (else
        (Rendering|SetActorHiddenInGame true)))))

(fn ConstructionScript)

(fn TurnonLight
  (params (Night :type Boolean)))