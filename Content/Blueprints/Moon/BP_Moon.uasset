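; BP_Moon is a moon actor with keyboard controls for phase and emission timelines and a configurable orbit offset.
; The construction script moves the actor to Center and sets the Sphere's relative location to Center plus OrbitDiameter along Y.
; Holding Z or X plays or reverses PhaseChanging, while holding C alternately plays or reverses EmissioonChanging.
; Neither timeline's output drives anything here, as the phase-to-yaw rotator is unused.
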(event EventBeginPlay)

(event Collision|EventActorBeginOverlap
  (params (OtherActor :type Actor%20Object%20Reference)))

(event EventTick
  (params (DeltaSeconds :type Float%20%28single-precision%29)))

(event Input|KeyboardEvents|Z
  (params (Key :type Key%20Structure :default "None"))
  (:Pressed
    (bind _newtrack_0 (Timeline|Phase%20Changing Play)))
  (:Released
    (Timeline|Phase%20Changing Stop)))

(event Input|KeyboardEvents|X
  (params (Key :type Key%20Structure :default "None"))
  (:Pressed
    (bind _newtrack_0 (Timeline|Phase%20Changing Reverse)))
  (:Released
    (Timeline|Phase%20Changing Stop)))

(event Input|KeyboardEvents|C
  (params (Key :type Key%20Structure :default "None"))
  (:Pressed
    (Utilities|FlowControl|FlipFlop
      (:A
        (Timeline|Emissioon%20Changing Play))
      (:B
        (Timeline|Emissioon%20Changing Reverse))))
  (:Released
    (Timeline|Emissioon%20Changing Stop)))

(fn ConstructionScript
  (Transformation|SetActorLocation (Variables|Default|Getcenter) false false)
  (Transformation|SetRelativeLocation (Variables|Default|GetSphere) (+ (Variables|Default|Getcenter) (Math|Vector|MakeVector 0.0 (Variables|Default|GetOrbitDiameter) 0.0)) false false))