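; BP_Car is a car actor that loops along a track spline, positioned as a function of shared time.
; Each Tick, it turns ParentTimeCore's time plus a per-car time offset, scaled by speed, into a distance wrapped by the rounded spline length.
; It teleports to that point, shifted sideways by Offset along the right vector, keeping its own Z.
; Its rotation comes from the spline's local-space rotation at that distance.
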(event EventBeginPlay)

(event Collision|EventActorBeginOverlap
  (params (OtherActor :type Actor%20Object%20Reference)))

(event EventTick
  (params (DeltaSeconds :type Float%20%28single-precision%29))
  (bind _parenttimecore (Variables|Default|GetParentTimeCore))
  (bind _trackspline (Variables|Default|GetTrackSpline))
  (bind _speed (Variables|Default|GetSpeed))
  (bind _offset (Variables|Default|GetOffset))
  (bind _timeoffset (Variables|EpochesandTime|GetTimeOffset))
  (bind _returnvalue (Transformation|GetActorLocation _trackspline))
  (bind _timevalue (Variables|/Script/SDProject.TimeCore|GetTimeValue _parenttimecore))
  (bind _spline (Variables|/Game/Blueprints/BP_Spline.BP_Spline_C|GetSpline _trackspline))
  (bind _returnvalue_2 (Spline|GetSplineLength _spline))
  (bind _returnvalue_3 (+ _timeoffset _timevalue))
  (bind _returnvalue_4 (Math|Float|Round _returnvalue_2))
  (bind _returnvalue_5 (* _speed _returnvalue_3))
  (bind _returnvalue_6 (Math|Integer|%(Integer) _returnvalue_5 _returnvalue_4))
  (bind _returnvalue_7 (Math|Conversions|ToFloat(Integer) _returnvalue_6))
  (bind _returnvalue_8 (Class|SplineComponent|GetRightVectoratDistanceAlongSpline _spline _returnvalue_7 "Local"))
  (bind _returnvalue_9 (Spline|GetLocationatDistanceAlongSpline _spline _returnvalue_7 "Local"))
  (bind _returnvalue_10 (* _returnvalue_8 _offset))
  (bind _returnvalue_11 (+ _returnvalue _returnvalue_9 _returnvalue_10))
  (Transformation|SetActorLocation (Math|Vector|MakeVector (.x _returnvalue_11) (.y _returnvalue_11) (.z (Transformation|GetActorLocation))) false true)
  (Transformation|SetActorRotation (Spline|GetRotationatDistanceAlongSpline _spline _returnvalue_7 "Local")))

(fn ConstructionScript)